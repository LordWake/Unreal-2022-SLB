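; Construction-script Blueprint for a spline-based wire prop in the Subway map, built from spline mesh segments.
; SplineMeshVar places segments either between spline points or at fixed Spacing intervals along the spline's length, with tangents scaled by TangentScale.
; WireVar selects among six spline mesh component variants, scaled by WireSize.
; Each segment gets two dynamic MI_Wire material instances with color, dirt, specular and roughness parameters, plus a TextureVar-selected texture set.
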(fn ConstructionScript
  (|Wire))
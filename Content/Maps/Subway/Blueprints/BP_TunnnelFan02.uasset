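; Subway tunnel fan Blueprint that continuously spins three fan components.
; Each Tick adds local pitch rotation to TunnelFan041, TunnelFan042 and TunnelFan043, each driven by its own speed variable.
; The rotation is a fixed step per frame without delta-time scaling, so spin speed varies with frame rate.
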(event EventTick
  (params (DeltaSeconds :type Float%20%28single-precision%29))
  ;[1 1 1] Fan Rotation
  (Transformation|AddLocalRotation (Variables|Default|GetTunnelFan041) (Math|Rotator|MakeRotator 0.0 (Variables|Default|GetRitation%20Speed) 0.0) false false)
  (Transformation|AddLocalRotation (Variables|Default|GetTunnelFan042) (Math|Rotator|MakeRotator 0.0 (Variables|Default|GetRitation%20Speed2) 0.0) false false)
  (Transformation|AddLocalRotation (Variables|Default|GetTunnelFan043) (Math|Rotator|MakeRotator 0.0 (Variables|Default|GetRitation%20Speed3) 0.0) false false))

(fn ConstructionScript)
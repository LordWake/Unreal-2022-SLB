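; BP_Train is a configurable subway train car assembled from static mesh components in its construction script.
; VagonVariant selects one of two body layouts, the second adding a mesh and shifting the doors at one end.
; Per-side position variables slide the twenty door leaves, and flags add optional front block, back block and merge meshes.
; A dynamic instance of MI_Train, shared across the parts, exposes color, roughness, specular, metal and emissive settings.
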(fn ConstructionScript
  (bind _position_r_door (Variables|Default|GetPosition%20R%20Door))
  (bind _position_front_door (Variables|Default|GetPosition%20Front%20Door))
  (bind _position_back_door (Variables|Default|GetPosition%20Back%20Door))
  (bind _position_l_door (Variables|Default|GetPosition%20L%20Door))
  (bind _returnvalue (Math|Vector|MakeVector 0.0 _position_back_door 0.0))
  (bind _returnvalue_2 (Math|Vector|MakeVector _position_r_door 0.0 0.0))
  (bind _returnvalue_3 (Math|Vector|MakeVector _position_l_door 0.0 0.0))
  ;[1 1 1] Add Mesh Component
  (Variables|Default|SetComponent%20Train%20Truck%201 0)
  (Variables|Default|SetComponent%20Train%20Truck%202 0)
  (Variables|Default|SetComponent%20Train%20Down 0)
  (Variables|Default|SetComponent%20Train%20Mesh%20Main 0)
  (Variables|Default|SetComponent%20Train%20Mesh%2001 0)
  (Variables|Default|SetComponent%20Train%20Mesh%2002 0)
  (Variables|Default|SetComponent%20Train%20Mesh%2003 0)
  (Variables|Default|SetComponent%20Train%20Mesh%2004 0)
  (Variables|Default|SetComponent%20Train%20Mesh%2005 0)
  (Variables|Default|SetComponent%20Train%20Mesh%2006 0)
  (Variables|Default|SetComponent%20Train%20Mesh%2007 0)
  (Variables|Default|SetComponent%20Train%20Mesh%2008 0)
  (Variables|Default|SetComponent%20Train%20Mesh%2009 0)
  (Variables|Default|SetComponent%20Train%20Mesh%2010 0)
  (Variables|Default|SetComponent%20Train%20Mesh%2011 0)
  (Variables|Default|SetComponent%20Train%20Mesh%2012 0)
  (Variables|Default|SetComponent%20Door%20Mesh%2001 0)
  (Variables|Default|SetComponent%20Door%20Mesh%2002 0)
  (Variables|Default|SetComponent%20Door%20Mesh%2003 0)
  (Variables|Default|SetComponent%20Door%20Mesh%2004 0)
  (Variables|Default|SetComponent%20Door%20Mesh%2005 0)
  (Variables|Default|SetComponent%20Door%20Mesh%2006 0)
  (Variables|Default|SetComponent%20Door%20Mesh%2007 0)
  (Variables|Default|SetComponent%20Door%20Mesh%2008 0)
  (Variables|Default|SetComponent%20Door%20Mesh%2009 0)
  (Variables|Default|SetComponent%20Door%20Mesh%2010 0)
  (Variables|Default|SetComponent%20Door%20Mesh%2011 0)
  (Variables|Default|SetComponent%20Door%20Mesh%2012 0)
  (Variables|Default|SetComponent%20Door%20Mesh%2013 0)
  (Variables|Default|SetComponent%20Door%20Mesh%2014 0)
  (Variables|Default|SetComponent%20Door%20Mesh%2015 0)
  (Variables|Default|SetComponent%20Door%20Mesh%2016 0)
  (Variables|Default|SetComponent%20Door%20Mesh%2017 0)
  (Variables|Default|SetComponent%20Door%20Mesh%2018 0)
  (Variables|Default|SetComponent%20Door%20Mesh%2019 0)
  (Variables|Default|SetComponent%20Door%20Mesh%2020 0)
  (Variables|Default|SetComponent%20Block%201 0)
  (Variables|Default|SetComponent%20Block%202 0)
  (Variables|Default|SetComponent%20Merge%201 0)
  (Variables|Default|SetComponent%20Merge%202 0)
  ;[1 1 1] Vagon mesh Variant
  (bind _returnvalue_4 (AddComponent|AddStaticMeshComponent false))
  (Variables|Default|SetComponent%20Train%20Truck%201 _returnvalue_4)
  (bind _returnvalue_5 (AddComponent|AddStaticMeshComponent false))
  (Variables|Default|SetComponent%20Train%20Truck%202 _returnvalue_5)
  (bind _returnvalue_6 (AddComponent|AddStaticMeshComponent false))
  (Variables|Default|SetComponent%20Train%20Down _returnvalue_6)
  (switch int (Variables|Default|GetVagonVariant)
    (:Default
      (bind _returnvalue_7 (AddComponent|AddStaticMeshComponent false :!label _label))
      (Variables|Default|SetComponent%20Train%20Mesh%20Main _returnvalue_7)
      (bind _returnvalue_8 (AddComponent|AddStaticMeshComponent false))
      (Variables|Default|SetComponent%20Train%20Mesh%2001 _returnvalue_8)
      (bind _returnvalue_9 (AddComponent|AddStaticMeshComponent false))
      (Variables|Default|SetComponent%20Train%20Mesh%2002 _returnvalue_9)
      (bind _returnvalue_10 (AddComponent|AddStaticMeshComponent false))
      (Variables|Default|SetComponent%20Train%20Mesh%2003 _returnvalue_10)
      (bind _returnvalue_11 (AddComponent|AddStaticMeshComponent false))
      (Variables|Default|SetComponent%20Train%20Mesh%2004 _returnvalue_11)
      (bind _returnvalue_12 (AddComponent|AddStaticMeshComponent false))
      (Variables|Default|SetComponent%20Train%20Mesh%2005 _returnvalue_12)
      (bind _returnvalue_13 (AddComponent|AddStaticMeshComponent false))
      (Variables|Default|SetComponent%20Train%20Mesh%2006 _returnvalue_13)
      (bind _returnvalue_14 (AddComponent|AddStaticMeshComponent false))
      (Variables|Default|SetComponent%20Train%20Mesh%2007 _returnvalue_14)
      (bind _returnvalue_15 (AddComponent|AddStaticMeshComponent false))
      (Variables|Default|SetComponent%20Train%20Mesh%2008 _returnvalue_15)
      (bind _returnvalue_16 (AddComponent|AddStaticMeshComponent false))
      (Variables|Default|SetComponent%20Train%20Mesh%2009 _returnvalue_16)
      (bind _returnvalue_17 (AddComponent|AddStaticMeshComponent false))
      (Variables|Default|SetComponent%20Train%20Mesh%2010 _returnvalue_17)
      (bind _returnvalue_18 (AddComponent|AddStaticMeshComponent false))
      (Variables|Default|SetComponent%20Train%20Mesh%2011 _returnvalue_18)
      (Variables|Default|SetDoor%20Local1 0.0)
      (Variables|Default|SetDoor%20Local2 0.0))
    (:0
      (goto _label))
    (:1
      (bind _returnvalue_19 (AddComponent|AddStaticMeshComponent false))
      (Variables|Default|SetComponent%20Train%20Mesh%20Main _returnvalue_19)
      (bind _returnvalue_20 (AddComponent|AddStaticMeshComponent false))
      (Variables|Default|SetComponent%20Train%20Mesh%2001 _returnvalue_20)
      (bind _returnvalue_21 (AddComponent|AddStaticMeshComponent false))
      (Variables|Default|SetComponent%20Train%20Mesh%2002 _returnvalue_21)
      (bind _returnvalue_22 (AddComponent|AddStaticMeshComponent false))
      (Variables|Default|SetComponent%20Train%20Mesh%2003 _returnvalue_22)
      (bind _returnvalue_23 (AddComponent|AddStaticMeshComponent false))
      (Variables|Default|SetComponent%20Train%20Mesh%2004 _returnvalue_23)
      (bind _returnvalue_24 (AddComponent|AddStaticMeshComponent false))
      (Variables|Default|SetComponent%20Train%20Mesh%2005 _returnvalue_24)
      (bind _returnvalue_25 (AddComponent|AddStaticMeshComponent false))
      (Variables|Default|SetComponent%20Train%20Mesh%2006 _returnvalue_25)
      (bind _returnvalue_26 (AddComponent|AddStaticMeshComponent false))
      (Variables|Default|SetComponent%20Train%20Mesh%2007 _returnvalue_26)
      (bind _returnvalue_27 (AddComponent|AddStaticMeshComponent false))
      (Variables|Default|SetComponent%20Train%20Mesh%2008 _returnvalue_27)
      (bind _returnvalue_28 (AddComponent|AddStaticMeshComponent false))
      (Variables|Default|SetComponent%20Train%20Mesh%2009 _returnvalue_28)
      (bind _returnvalue_29 (AddComponent|AddStaticMeshComponent false))
      (Variables|Default|SetComponent%20Train%20Mesh%2010 _returnvalue_29)
      (bind _returnvalue_30 (AddComponent|AddStaticMeshComponent false))
      (Variables|Default|SetComponent%20Train%20Mesh%2011 _returnvalue_30)
      (bind _returnvalue_31 (AddComponent|AddStaticMeshComponent false))
      (bind _output_get (Variables|Default|SetComponent%20Train%20Mesh%2012 _returnvalue_31))
      (Rendering|Material|SetMaterial _output_get 0 (stale _returnvalue_56))
      (Variables|Default|SetDoor%20Local1 121.5)
      (Variables|Default|SetDoor%20Local2 4e+01)))
  ;[1 1 1] Door Position
  (bind _returnvalue_32 (AddComponent|AddStaticMeshComponent false (Math|Conversions|ToTransform(Vector) (- "905.000000, 0, 0" _returnvalue))))
  (Variables|Default|SetComponent%20Door%20Mesh%2001 _returnvalue_32)
  (bind _returnvalue_33 (AddComponent|AddStaticMeshComponent false (Math|Conversions|ToTransform(Vector) (+ "905.000000, 0, 0" _returnvalue))))
  (Variables|Default|SetComponent%20Door%20Mesh%2002 _returnvalue_33)
  (bind _returnvalue_34 (AddComponent|AddStaticMeshComponent false (Math|Transform|MakeTransform (+ "-784.000000, 0, 0" (Math|Vector|MakeVector (- 0.0 (Variables|Default|GetDoor%20Local1)) _position_front_door 0.0)) "0,180.000000, 0")))
  (Variables|Default|SetComponent%20Door%20Mesh%2003 _returnvalue_34)
  (bind _returnvalue_35 (AddComponent|AddStaticMeshComponent false (Math|Transform|MakeTransform (- "-784.000000, 0, 0" (Math|Vector|MakeVector (Variables|Default|GetDoor%20Local1) _position_front_door 0.0)) "0,180.000000, 0")))
  (Variables|Default|SetComponent%20Door%20Mesh%2004 _returnvalue_35)
  (bind _returnvalue_36 (AddComponent|AddStaticMeshComponent false (Math|Conversions|ToTransform(Vector) (- "-635.000000, 0, 0" (Math|Vector|MakeVector (+ (Variables|Default|GetDoor%20Local2) _position_r_door) 0.0 0.0)))))
  (Variables|Default|SetComponent%20Door%20Mesh%2005 _returnvalue_36)
  (bind _returnvalue_37 (AddComponent|AddStaticMeshComponent false (Math|Conversions|ToTransform(Vector) (+ (Math|Vector|MakeVector (+ (- 0.0 (Variables|Default|GetDoor%20Local2)) _position_r_door) 0.0 0.0) "-635.000000, 0, 0"))))
  (Variables|Default|SetComponent%20Door%20Mesh%2006 _returnvalue_37)
  (bind _returnvalue_38 (AddComponent|AddStaticMeshComponent false (Math|Conversions|ToTransform(Vector) (- "-225.000000, 0, 0" _returnvalue_2))))
  (Variables|Default|SetComponent%20Door%20Mesh%2007 _returnvalue_38)
  (bind _returnvalue_39 (AddComponent|AddStaticMeshComponent false (Math|Conversions|ToTransform(Vector) (+ _returnvalue_2 "-225.000000, 0, 0"))))
  (Variables|Default|SetComponent%20Door%20Mesh%2008 _returnvalue_39)
  (bind _returnvalue_40 (AddComponent|AddStaticMeshComponent false (Math|Conversions|ToTransform(Vector) (- "225.000000, 0, 0" _returnvalue_2))))
  (Variables|Default|SetComponent%20Door%20Mesh%2009 _returnvalue_40)
  (bind _returnvalue_41 (AddComponent|AddStaticMeshComponent false (Math|Conversions|ToTransform(Vector) (+ _returnvalue_2 "225.000000, 0, 0"))))
  (Variables|Default|SetComponent%20Door%20Mesh%2010 _returnvalue_41)
  (bind _returnvalue_42 (AddComponent|AddStaticMeshComponent false (Math|Conversions|ToTransform(Vector) (- "675.000000, 0, 0" _returnvalue_2))))
  (Variables|Default|SetComponent%20Door%20Mesh%2011 _returnvalue_42)
  (bind _returnvalue_43 (AddComponent|AddStaticMeshComponent false (Math|Conversions|ToTransform(Vector) (+ _returnvalue_2 "675.000000, 0, 0"))))
  (Variables|Default|SetComponent%20Door%20Mesh%2012 _returnvalue_43)
  (bind _returnvalue_44 (AddComponent|AddStaticMeshComponent false (Math|Transform|MakeTransform (+ (Math|Vector|MakeVector (+ (- 0.0 (Variables|Default|GetDoor%20Local2)) _position_l_door) 0.0 0.0) "-635.000000, 0, 0") "0,180.000000, 0")))
  (Variables|Default|SetComponent%20Door%20Mesh%2013 _returnvalue_44)
  (bind _returnvalue_45 (AddComponent|AddStaticMeshComponent false (Math|Transform|MakeTransform (- "-635.000000, 0, 0" (Math|Vector|MakeVector (+ (Variables|Default|GetDoor%20Local2) _position_l_door) 0.0 0.0)) "0,180.000000, 0")))
  (Variables|Default|SetComponent%20Door%20Mesh%2014 _returnvalue_45)
  (bind _returnvalue_46 (AddComponent|AddStaticMeshComponent false (Math|Transform|MakeTransform (+ _returnvalue_3 "-225.000000, 0, 0") "0,180.000000, 0")))
  (Variables|Default|SetComponent%20Door%20Mesh%2015 _returnvalue_46)
  (bind _returnvalue_47 (AddComponent|AddStaticMeshComponent false (Math|Transform|MakeTransform (- "-225.000000, 0, 0" _returnvalue_3) "0,180.000000, 0" "1.000000,1,1")))
  (Variables|Default|SetComponent%20Door%20Mesh%2016 _returnvalue_47)
  (bind _returnvalue_48 (AddComponent|AddStaticMeshComponent false (Math|Transform|MakeTransform (+ _returnvalue_3 "225.000000, 0, 0") "0,180.000000, 0")))
  (Variables|Default|SetComponent%20Door%20Mesh%2017 _returnvalue_48)
  (bind _returnvalue_49 (AddComponent|AddStaticMeshComponent false (Math|Transform|MakeTransform (- "225.000000, 0, 0" _returnvalue_3) "0,180.000000, 0")))
  (Variables|Default|SetComponent%20Door%20Mesh%2018 _returnvalue_49)
  (bind _returnvalue_50 (AddComponent|AddStaticMeshComponent false (Math|Transform|MakeTransform (+ _returnvalue_3 "675.000000, 0, 0") "0,180.000000, 0")))
  (Variables|Default|SetComponent%20Door%20Mesh%2019 _returnvalue_50)
  (bind _returnvalue_51 (AddComponent|AddStaticMeshComponent false (Math|Transform|MakeTransform (- "675.000000, 0, 0" _returnvalue_3) "0,180.000000, 0" "1.000000,1,1")))
  (Variables|Default|SetComponent%20Door%20Mesh%2020 _returnvalue_51)
  ;[1 1 1] Meshes
  (if (Variables|Default|GetBlockFrontAdd)
    (bind _returnvalue_52 (AddComponent|AddStaticMeshComponent false))
    (bind _output_get_2 (Variables|Default|SetComponent%20Block%201 _returnvalue_52))
    (Rendering|Material|SetMaterial _output_get_2 0 (stale _returnvalue_56)))
  (if (Variables|Default|GetBlockBackAdd)
    (bind _returnvalue_53 (AddComponent|AddStaticMeshComponent false))
    (bind _output_get_3 (Variables|Default|SetComponent%20Block%202 _returnvalue_53))
    (Rendering|Material|SetMaterial _output_get_3 0 (stale _returnvalue_56)))
  (if (Variables|Default|GetTrainMergeAdd)
    (bind _returnvalue_54 (AddComponent|AddStaticMeshComponent false))
    (bind _output_get_4 (Variables|Default|SetComponent%20Merge%201 _returnvalue_54))
    (bind _returnvalue_55 (AddComponent|AddStaticMeshComponent false))
    (bind _output_get_5 (Variables|Default|SetComponent%20Merge%202 _returnvalue_55))
    (Rendering|Material|SetMaterial _output_get_4 0 (stale _returnvalue_56)))
  ;[1 1 1] Material
  (bind _returnvalue_56 (Rendering|Material|CreateDynamicMaterialInstance (Variables|Default|GetComponent%20Train%20Mesh%20Main) 0 "/Game/Maps/Subway/Materials/Train/MI_Train.MI_Train" "None" :!class /Script/Engine.PrimitiveComponent))
  (Rendering|Material|SetMaterial (Variables|Default|GetComponent%20Train%20Truck%201) 0 _returnvalue_56)
  (Rendering|Material|SetVectorParameterValue _returnvalue_56 "additional diffuse color" (Variables|Default|GetTrain%20Color) :!class /Script/Engine.MaterialInstanceDynamic)
  (Rendering|Material|SetVectorParameterValue _returnvalue_56 "metall color" (Variables|Default|GetMetall%20Color) :!class /Script/Engine.MaterialInstanceDynamic)
  (Rendering|Material|SetScalarParameterValue _returnvalue_56 "Roughness" (Variables|Default|GetRoughness) :!class /Script/Engine.MaterialInstanceDynamic)
  (Rendering|Material|SetScalarParameterValue _returnvalue_56 "spec" (Variables|Default|GetSpecular) :!class /Script/Engine.MaterialInstanceDynamic)
  (Rendering|Material|SetScalarParameterValue _returnvalue_56 "metall Roughness" (Variables|Default|GetMetall%20Roughness) :!class /Script/Engine.MaterialInstanceDynamic)
  (Rendering|Material|SetScalarParameterValue _returnvalue_56 "metall Contrast" (Variables|Default|GetMetall%20Contrast) :!class /Script/Engine.MaterialInstanceDynamic)
  (Rendering|Material|SetScalarParameterValue _returnvalue_56 "Emmisive Str" (Variables|Default|GetEmmisive) :!class /Script/Engine.MaterialInstanceDynamic))
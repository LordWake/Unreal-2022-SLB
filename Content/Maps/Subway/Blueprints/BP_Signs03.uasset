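; Hanging subway sign actor with two cables and two physics constraints that can be cut loose independently.
; On BeginPlay, each enabled break flag detaches its cable end and breaks the matching constraint.
; An impulse is then applied to the sign mesh unconditionally to start it swinging or falling.
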(event EventBeginPlay
  ;[1 1 1] Break Constraint
  (if (Variables|Default|GetBreak%20Constraint%201)
    (Variables|/Script/CableComponent.CableComponent|SetbAttachEnd (Variables|Default|GetCable1) false)
    (Class|PhysicsConstraintComponent|BreakConstraint (Variables|Components|GetConstL1)))
  (if (Variables|Default|GetBreak%20Constraint%202)
    (Variables|/Script/CableComponent.CableComponent|SetbAttachEnd (Variables|Default|GetCable2) false)
    (Class|PhysicsConstraintComponent|BreakConstraint (Variables|Components|GetConstL2)))
  (Physics|AddImpulse (Variables|Components|GetSigns) "1000.000000,1000.000000,1000.000000" "None" false))

(fn ConstructionScript)
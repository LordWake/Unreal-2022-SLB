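; BP_PoliceLine is a spline-based police line prop that builds its meshes in the Construction Script.
; It steps along the spline at a set spacing, adding one spline mesh per step from one of three component templates chosen by LineVar.
; Each segment takes its endpoints and scaled tangents from the spline.
; Each also gets its own dynamic instance of MI_PoliceLine with adjustable color, specular and roughness.
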(fn ConstructionScript
  (bind _spline (Variables|Default|GetSpline))
  (bind _spacing (Variables|Default|GetSpacing))
  (bind _tangentscale (Variables|Default|GetTangentScale))
  (Variables|Components|SetComponent%201 0)
  ;[1 1 1] Spline Point Position
  (for _index (range 0 (.ReturnValue (Math|Float|Division(WholeandRemainder) (Spline|GetSplineLength _spline) _spacing)))
    ;[1 1 1] Mesh Variant
    (switch int (Variables|Default|GetLineVar)
      (:Default
        (bind _returnvalue (AddComponent|AddSplineMeshComponent false :!label _label))
        (Variables|Components|SetComponent%201 _returnvalue))
      (:0
        (goto _label))
      (:1
        (bind _returnvalue_2 (AddComponent|AddSplineMeshComponent false))
        (Variables|Components|SetComponent%201 _returnvalue_2))
      (:2
        (bind _returnvalue_3 (AddComponent|AddSplineMeshComponent false))
        (Variables|Components|SetComponent%201 _returnvalue_3)))
    (SplineMesh|SetStartandEnd (Variables|Components|GetComponent%201) (Spline|GetLocationatDistanceAlongSpline _spline (* _index _spacing) "Local") (* (Spline|GetDirectionatDistanceAlongSpline _spline (* _index _spacing) "Local") _tangentscale) (Spline|GetLocationatDistanceAlongSpline _spline (+ (* _index _spacing) _spacing) "Local") (* (Spline|GetDirectionatDistanceAlongSpline _spline (+ (* _index _spacing) _spacing) "Local") _tangentscale) true :!class /Script/Engine.SplineMeshComponent)
    ;[1 1 1] Material
    (bind _returnvalue_4 (Rendering|Material|CreateDynamicMaterialInstance "/Game/Maps/Subway/Materials/Blueprint/MI_PoliceLine.MI_PoliceLine" "None" :!class /Script/Engine.KismetMaterialLibrary))
    (Rendering|Material|SetMaterial (Variables|Components|GetComponent%201) 0 _returnvalue_4)
    (Rendering|Material|SetVectorParameterValue _returnvalue_4 "diffuse color" (Variables|Default|GetColor) :!class /Script/Engine.MaterialInstanceDynamic)
    (Rendering|Material|SetScalarParameterValue _returnvalue_4 "Specular" (Variables|Default|GetSpecular) :!class /Script/Engine.MaterialInstanceDynamic)
    (Rendering|Material|SetScalarParameterValue _returnvalue_4 "Roughness" (Variables|Default|GetRoughness) :!class /Script/Engine.MaterialInstanceDynamic)))
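; Third-person player character Blueprint that drives smooth camera transitions for cover, aiming and sprinting.
; Three events each play a timeline forward when their state turns on and reverse it when off, lerping a camera property.
; Cover blends FOV from default to a cover value, and aiming blends from current FOV to the equipped weapon's zoom FOV.
; Sprinting lengthens the spring arm to pull the camera back.
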(event EventPlayerIsSprinting
  (params (bPlayerIsSprinting :type Boolean))
  ;[0 0 0] Zoom Sprint
  (if bPlayerIsSprinting
    (bind _sprinttime (Timeline|Sprint%20TimeLine Play)
      (:Update
        (Variables|/Script/Engine.SpringArmComponent|SetTargetArmLength (Variables|Default|GetSpringArmComponent) (Math|Float|Lerp 1.5e+02 2.5e+02 _sprinttime))))
    (else
      (Timeline|Sprint%20TimeLine Reverse))))

(event EventSetFOV
  (params (bIsAiming :type Boolean))
  ;[0 0 0] Zoom Aim
  (if bIsAiming
    (bind _zoomtime (Timeline|Zoom%20TimeLine Play)
      (:Update
        (Camera|SetFieldOfView (Variables|Default|GetCameraComponent) (Math|Float|Lerp (Variables|Default|GetCurrentFOVValue) (Variables|/Script/SmellsLikeBlood.BaseWeapon|GetZoomFOV (Variables|Default|GetEquippedWeapon)) _zoomtime))))
    (else
      (Timeline|Zoom%20TimeLine Reverse))))

(event EventSetCoverFOV
  (params (bOnCover :type Boolean))
  ;[0 0 0] CoverAim
  (if bOnCover
    (bind _zoomtime (Timeline|Cover%20TimeLine Play)
      (:Update
        (Camera|SetFieldOfView (Variables|Default|GetCameraComponent) (Math|Float|Lerp (Variables|Default|GetDefaultFOVValue) (Variables|Default|GetCoverFOVValue) _zoomtime))))
    (else
      (Timeline|Cover%20TimeLine Reverse))))

(fn ConstructionScript)
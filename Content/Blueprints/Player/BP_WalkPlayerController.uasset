(event EventReloadLevelfromPause
  (params (bGoToMainMenu :type Boolean))
  ;[1 0 0] Reload Current Level from Pause Menu
  (bind _returnvalue (UserInterface|CreateWidget "/Game/Widgets/WBP/LevelIntro/LoadingScreen/WBP_LoadingScreen.WBP_LoadingScreen_C" self))
  (UserInterface|Viewport|AddtoViewport _returnvalue 0)
  (Utilities|FlowControl|Delay 1.5)
  (bind _asbp_slb_game_instance (Utilities|Casting|CastToBP_SLB_GameInstance (Game|GetGameInstance)))
  (Class|WalkPlayerController|GameonPause false)
  (if bGoToMainMenu
    (Game|OpenLevel(byName) "MainMenu")
    (else
      (Game|OpenLevel(byName) (Variables|/Script/SmellsLikeBlood.SaveGameMaster|GetLevelToLoad (Variables|/Script/SmellsLikeBlood.SLB_GameInstance|GetOriginalSaveFile _asbp_slb_game_instance))))))

(event EventGameonDialogueMode
  (params (bEnableDialogue :type Boolean) (DialogeLevelValue :type Integer) (DialogueIndexValue :type Integer))
  (bind _dialogueui (Variables|Default|GetDialogueUI))
  ;[0 0.9702 1] Dialogues
  (Class|WalkPlayerController|GameonPause false)
  (if bEnableDialogue
    (Game|SetGamePaused true)
    (Widget|SetVisibility _dialogueui "Visible")
    (Default|DialogueManager _dialogueui DialogeLevelValue DialogueIndexValue)
    (Input|SetInputModeUIOnly self (Variables|Default|GetDialogueUI) "LockOnCapture")
    (else
      (Widget|SetVisibility (Variables|Default|GetDialogueUI) "Hidden")
      (Class|WalkPlayerController|GameonPause false)
      (Input|SetInputModeGameOnly self))))

(event EventCreateandSetPauseUI
  ;[1 0.4297 0] Create and Set UI
  (bind _returnvalue (UserInterface|CreateWidget "/Game/Widgets/WBP/WBP_Pause.WBP_Pause_C" self))
  (Variables|Default|SetPauseUI _returnvalue))

(event EventGameonPause
  (params (bOnPause :type Boolean))
  (bind _pauseui (Variables|Default|GetPauseUI))
  ;[0 0 0] Pause UI
  (if bOnPause
    (Game|SetGamePaused true)
    (UserInterface|Viewport|AddtoViewport _pauseui 0)
    (Input|SetInputModeUIOnly self _pauseui "LockOnCapture")
    (else
      (Game|SetGamePaused false)
      (Widget|RemovefromParent _pauseui)
      (Input|SetInputModeGameOnly self))))

(event EventCreateandSetDialogueUI
  ;[1 0.4297 0] Create and Set UI
  (bind _returnvalue (UserInterface|CreateWidget "/Game/Widgets/WBP/WBP_Dialogue.WBP_Dialogue_C" self))
  (bind _output_get (Variables|Default|SetDialogueUI _returnvalue))
  (UserInterface|Viewport|AddtoViewport _output_get 0)
  (Widget|SetVisibility _output_get "Hidden"))

(fn ConstructionScript)
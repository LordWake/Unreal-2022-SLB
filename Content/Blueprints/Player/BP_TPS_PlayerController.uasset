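; Third-person shooter player controller that owns the player's UI and switches between gameplay, pause, dialogue and death-screen states.
; It creates the gameplay, dialogue and pause widgets, toggling visibility, game pause and input mode between them.
; HUD events forward health, heat, slow-time, crosshair and weapon-slot updates to the gameplay widget.
; It also hides weapons for cinematics and shows a loading screen before reloading the saved level or opening the main menu.
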(event Custom|HidePlayerWeaponsOnCinematic
  (params (Hide :type Boolean))
  (bind _self self)
  (bind _playercharacter (Variables|Default|GetPlayerCharacter))
  (bind _sniperrifleslot (Variables|/Script/SmellsLikeBlood.TPS_PlayerCharacter|GetSniperRifleSlot _playercharacter))
  (bind _shotgunslot (Variables|/Script/SmellsLikeBlood.TPS_PlayerCharacter|GetShotgunSlot _playercharacter))
  ;[0 0.4926 1] Hide player weapons on cinematics.
  (Rendering|SetActorHiddenInGame (Variables|/Script/SmellsLikeBlood.TPS_PlayerCharacter|GetEquippedWeapon _playercharacter) Hide)
  (Rendering|SetActorHiddenInGame (Variables|/Script/SmellsLikeBlood.TPS_PlayerCharacter|GetAssaultRifleSlot _playercharacter) Hide)
  (Utilities|IsValid _shotgunslot
    (:Is%20Valid
      (Rendering|SetActorHiddenInGame _shotgunslot Hide))
    (:Is%20Not%20Valid
      _))
  (Utilities|IsValid _sniperrifleslot
    (:Is%20Valid
      (Rendering|SetActorHiddenInGame _sniperrifleslot Hide)
      (if Hide
        (Input|DisableInput _self)
        (else
          (Input|EnableInput _self))))))

(event EventSetHUDonScreen
  ;[0 0 0] Create UI
  (Utilities|FlowControl|Sequence
    (:then_0
      (bind _returnvalue (UserInterface|CreateWidget "/Game/Widgets/WBP/WBP_Gameplay.WBP_Gameplay_C" self))
      (bind _output_get (Variables|Default|SetGameplayUI _returnvalue))
      (UserInterface|Viewport|AddtoViewport _output_get 0)
      (Variables|/Game/Widgets/WBP/WBP_Gameplay.WBP_Gameplay_C|SetPlayerControllerRef _output_get self)
      (Class|TPSPlayerController|ShoworHideAllGameplayUI true))
    (:then_1
      (bind _returnvalue_2 (UserInterface|CreateWidget "/Game/Widgets/WBP/WBP_Dialogue.WBP_Dialogue_C" self))
      (bind _output_get_2 (Variables|Default|SetDialogueUI _returnvalue_2))
      (UserInterface|Viewport|AddtoViewport _output_get_2 0)
      (Widget|SetVisibility _output_get_2 "Hidden"))
    (:then_2
      (bind _returnvalue_3 (UserInterface|CreateWidget "/Game/Widgets/WBP/WBP_Pause.WBP_Pause_C" self))
      (Variables|Default|SetPauseUI _returnvalue_3))))

(event EventSetCrossHairVisibility
  (params (bIsCrosshairVisible :type Boolean))
  ;[1 0 0] Cross Hair
  (Default|SetCrossHairVisibility (Variables|Default|GetGameplayUI) bIsCrosshairVisible))

(event EventShowWeaponAvailabletoPickHUD
  (params (WeaponIndex :type Integer%20%28by%20ref%29))
  ;[0 0 0] Show Weapon Available To Pick
  (Default|OnTakeWeapon (Variables|Default|GetGameplayUI) WeaponIndex))

(event EventSetSlowTimeHUDValue
  (params (SlowTimeValue :type Float%20%28single-precision%29))
  ;[0.1317 0.85 1] Life, Overheat and SlowTime bars value
  (Default|UpdateSlowTimeValue (Variables|Default|GetGameplayUI) SlowTimeValue))

(event EventShoworHideAllGameplayUI
  (params (bHideTheUI :type Boolean))
  (bind _self self)
  (bind _gameplayui (Variables|Default|GetGameplayUI))
  ;[1 0.8922 0.1458] Show/Hide UI
  (if bHideTheUI
    (Widget|SetVisibility _gameplayui "Hidden")
    (Input|SetInputModeUIOnly _self _gameplayui "DoNotLock")
    (else
      (Widget|SetVisibility _gameplayui "Visible")
      (Input|SetInputModeGameOnly _self))))

(event EventGameonPause
  (params (bOnPause :type Boolean))
  (bind _pauseui (Variables|Default|GetPauseUI))
  ;[0 0 0] Pause
  (if bOnPause
    (Widget|SetVisibility (Variables|Default|GetGameplayUI) "Hidden")
    (Game|SetGamePaused true)
    (UserInterface|Viewport|AddtoViewport _pauseui 0)
    (Input|SetInputModeUIOnly self _pauseui "LockOnCapture")
    (else
      (Game|SetGamePaused false)
      (Widget|RemovefromParent (Variables|Default|GetPauseUI))
      (Widget|SetVisibility (Variables|Default|GetGameplayUI) "Visible")
      (Input|SetInputModeGameOnly self))))

(event EventGameonDialogueMode
  (params (bEnableDialogue :type Boolean) (DialogeLevelValue :type Integer) (DialogueIndexValue :type Integer))
  (bind _dialogueui (Variables|Default|GetDialogueUI))
  ;[0.3293 1 0] Dialogues
  (Class|TPSPlayerController|SetPlayertoDialogueMode)
  (Class|TPSPlayerController|GameonPause false)
  (if bEnableDialogue
    (Widget|SetVisibility (Variables|Default|GetGameplayUI) "Hidden")
    (Game|SetGamePaused true)
    (Widget|SetVisibility _dialogueui "Visible")
    (Default|DialogueManager _dialogueui DialogeLevelValue DialogueIndexValue)
    (Input|SetInputModeUIOnly self (Variables|Default|GetDialogueUI) "LockOnCapture")
    (else
      (Widget|SetVisibility (Variables|Default|GetDialogueUI) "Hidden")
      (Widget|SetVisibility (Variables|Default|GetGameplayUI) "Visible")
      (Class|TPSPlayerController|GameonPause false)
      (Input|SetInputModeGameOnly self))))

(event EventPlayerIsDeadUISet
  (bind _self self)
  ;[1 0 0] Player's Dead
  (Utilities|FlowControl|Delay 3.0)
  (Widget|SetVisibility (Variables|Default|GetGameplayUI) "Hidden")
  (Game|SetGamePaused true)
  (bind _returnvalue (UserInterface|CreateWidget "/Game/Widgets/WBP/WBP_DeathScreen.WBP_DeathScreen_C" _self))
  (UserInterface|Viewport|AddtoViewport _returnvalue 0)
  (Input|SetInputModeUIOnly _self _returnvalue "LockOnCapture"))

(event EventReloadLevelfromPause
  (params (bGoToMainMenu :type Boolean))
  ;[1 0.4096 0.2069] Reload current level from Pause Menu
  (Widget|RemovefromParent (Variables|Default|GetGameplayUI))
  (bind _returnvalue (UserInterface|CreateWidget "/Game/Widgets/WBP/LevelIntro/LoadingScreen/WBP_LoadingScreen.WBP_LoadingScreen_C" self))
  (UserInterface|Viewport|AddtoViewport _returnvalue 0)
  (Utilities|FlowControl|Delay 3.0)
  (bind _asbp_slb_game_instance (Utilities|Casting|CastToBP_SLB_GameInstance (Game|GetGameInstance)))
  (Class|TPSPlayerController|GameonPause false)
  (if bGoToMainMenu
    (Game|OpenLevel(byName) "MainMenu")
    (else
      (Game|OpenLevel(byName) (Variables|/Script/SmellsLikeBlood.SaveGameMaster|GetLevelToLoad (Variables|/Script/SmellsLikeBlood.SLB_GameInstance|GetOriginalSaveFile _asbp_slb_game_instance))))))

(event EventStrippersDialogueWarning
  ;[0 0 0] Strippers Warning
  (Class|TPSPlayerController|GameonDialogueMode true 3))

(event EventSetLifeHUDValue
  (params (LifePercent :type Float%20%28single-precision%29))
  ;[0.1317 0.85 1] Life, Overheat and SlowTime bars value
  (Default|SetLifePercentonScreen (Variables|Default|GetGameplayUI) LifePercent))

(event EventSetWeaponHeatHUDValue
  (params (HeatAmount :type Float%20%28single-precision%29))
  ;[0.1317 0.85 1] Life, Overheat and SlowTime bars value
  (Default|SetHeatAmount (Variables|Default|GetGameplayUI) HeatAmount))

(event EventSetWeaponIsOverHeatedHUDValue
  (params (bOverHeatedWeapon :type Boolean))
  ;[0 0 0] Weapons Misc
  (Default|SetOverheatText (Variables|Default|GetGameplayUI) bOverHeatedWeapon))

(event EventSetCurrentWeaponHUD
  (params (CurrentWeaponIndex :type Integer%20%28by%20ref%29))
  ;[0 0 0] Weapons Misc
  (Default|SetCurrentWeapononHUD (Variables|Default|GetGameplayUI) CurrentWeaponIndex))

(event EventSetCrossHairColor
  (params (bIsEnemyOnTarget :type Boolean))
  ;[1 0 0] Cross Hair
  (Default|SetCrossHairColor (Variables|Default|GetGameplayUI) bIsEnemyOnTarget))

(event EventSetHitmarkHUD
  ;[1 0 0] Cross Hair
  (Default|PlayHitmark (Variables|Default|GetGameplayUI)))

(event EventSetWeaponSlotsHUD
  (bind _gameplayui (Variables|Default|GetGameplayUI))
  (bind _playercharacter (Variables|Default|GetPlayerCharacter))
  (bind _shotgunslot (Variables|/Script/SmellsLikeBlood.TPS_PlayerCharacter|GetShotgunSlot _playercharacter))
  (bind _sniperrifleslot (Variables|/Script/SmellsLikeBlood.TPS_PlayerCharacter|GetSniperRifleSlot _playercharacter))
  (bind _assaultrifleslot (Variables|/Script/SmellsLikeBlood.TPS_PlayerCharacter|GetAssaultRifleSlot _playercharacter))
  ;[1 0 0] Change Weapon Slots
  (Utilities|FlowControl|Sequence
    (:then_0
      (Utilities|IsValid _assaultrifleslot
        (:Is%20Valid
          (switch Utilities|FlowControl|Switch|SwitchonEAllWeaponTypes (Variables|/Script/SmellsLikeBlood.AssaultRifle|GetThisWeaponType _assaultrifleslot)
            (:AssaultRifleWeapon
              (Default|SetRifleSlotHUD _gameplayui))
            (:LegendaryAssaultRifle
              (Default|SetRifleSlotHUD _gameplayui 1))))))
    (:then_1
      (Utilities|IsValid _shotgunslot
        (:Is%20Valid
          (switch Utilities|FlowControl|Switch|SwitchonEAllWeaponTypes (Variables|/Script/SmellsLikeBlood.Shotgun|GetThisWeaponType _shotgunslot)
            (:ShotgunWeapon
              (Default|SetShotgunSlotHUD _gameplayui 1))
            (:LegendaryShotgun
              (Default|SetShotgunSlotHUD _gameplayui 2))))
        (:Is%20Not%20Valid
          (Default|SetShotgunSlotHUD _gameplayui))))
    (:then_2
      (Utilities|IsValid _sniperrifleslot
        (:Is%20Valid
          (switch Utilities|FlowControl|Switch|SwitchonEAllWeaponTypes (Variables|/Script/SmellsLikeBlood.SniperRifleWeapon|GetThisWeaponType _sniperrifleslot)
            (:SniperRifleWeapon
              (Default|SetSniperSlotHUD _gameplayui 1))
            (:LegendarySniperRifle
              (Default|SetSniperSlotHUD _gameplayui 2))))
        (:Is%20Not%20Valid
          (Default|SetSniperSlotHUD _gameplayui))))))

(event EventShowWeaponSwitchHUD
  (bind _gameplayui (Variables|Default|GetGameplayUI))
  ;[0 0 0] Switch Weapons HUD
  (switch Utilities|FlowControl|Switch|SwitchonECurrentWeapon (Variables|/Script/SmellsLikeBlood.TPS_PlayerCharacter|GetCurrentWeapon (Variables|Default|GetPlayerCharacter))
    (:AssaultRifleWeapon
      (Default|ShowWeaponSwitch _gameplayui))
    (:LegendaryAssaultRifle
      (Default|ShowWeaponSwitch _gameplayui))
    (:ShotgunWeapon
      (Default|ShowWeaponSwitch _gameplayui 1))
    (:LegendaryShotgun
      (Default|ShowWeaponSwitch _gameplayui 1))
    (:SniperRifleWeapon
      (Default|ShowWeaponSwitch _gameplayui 2))
    (:LegendarySniperWeapon
      (Default|ShowWeaponSwitch _gameplayui 2))))

(fn ConstructionScript)

(fn CheckifWeHavetoPlayCinematic)
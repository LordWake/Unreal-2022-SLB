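; Main menu player controller that creates the menu, settings, controls and credits widgets and swaps them on screen for navigation.
; The menu shows a new-game or continue variant depending on whether the saved LevelToLoad in BP_SLB_GameInstance equals the initial level name.
; Starting play disables input, shows a loading screen, waits briefly, stops player movement, then opens the saved level by name.
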(event EventChangetoPlayableLevel
  ;[0 1 0.2676] Change Level
  (Input|DisableInput self)
  (bind _returnvalue (UserInterface|CreateWidget "/Game/Widgets/WBP/LevelIntro/LoadingScreen/WBP_LoadingScreen.WBP_LoadingScreen_C" self))
  (UserInterface|Viewport|AddtoViewport _returnvalue 0)
  (Widget|RemovefromParent (Variables|Default|GetMenuWidget))
  (Utilities|FlowControl|Delay 2.0)
  (Class|MenuController|StopPlayerMovement)
  (bind _asbp_slb_game_instance (Utilities|Casting|CastToBP_SLB_GameInstance (Game|GetGameInstance)))
  (Game|OpenLevel(byName) (Variables|/Script/SmellsLikeBlood.SaveGameMaster|GetLevelToLoad (Variables|/Script/SmellsLikeBlood.SLB_GameInstance|GetOriginalSaveFile _asbp_slb_game_instance))))

(event EventBacktoMainMenuHUD
  ;[0 1 0.5286] Settings, Controls and Back To Main Menu. Basically, UI Navigation Flow
  (Widget|RemovefromParent (Variables|Default|GetCredits))
  (Widget|RemovefromParent (Variables|Default|GetMenuSettings))
  (Widget|RemovefromParent (Variables|Default|GetControls))
  (UserInterface|Viewport|AddtoViewport (Variables|Default|GetMenuWidget) 0)
  (Audio|PlaySound2D "/Game/Sounds/SFX/UI/S_UI_Back_Cue.S_UI_Back_Cue" 1.0 1.0 0.0 0 0))

(event EventSetHUDonScreen
  ;[0.9376 1 0.009724] Set Main HUD On Screen
  (bind _asbp_slb_game_instance (Utilities|Casting|CastToBP_SLB_GameInstance (Game|GetGameInstance)))
  (if (Utilities|Name|Equal(Name) (Variables|/Script/SmellsLikeBlood.SaveGameMaster|GetLevelToLoad (Variables|/Script/SmellsLikeBlood.SLB_GameInstance|GetOriginalSaveFile _asbp_slb_game_instance)) (Variables|Default|GetInitialLevelName))
    (Variables|Default|SetMainWidgetClass "/Game/Widgets/WBP/WBP_MainMenu.WBP_MainMenu_C")
    (else
      (Variables|Default|SetMainWidgetClass "/Game/Widgets/WBP/WBP_MainMenuContinue.WBP_MainMenuContinue_C")))
  (bind _returnvalue (UserInterface|CreateWidget (Variables|Default|GetMainWidgetClass) self))
  (bind _output_get (Variables|Default|SetMenuWidget _returnvalue))
  (UserInterface|Viewport|AddtoViewport _output_get 0)
  (bind _returnvalue_2 (UserInterface|CreateWidget "/Game/Widgets/WBP/WBP_Settings.WBP_Settings_C" self))
  (Variables|Default|SetMenuSettings _returnvalue_2)
  (bind _returnvalue_3 (UserInterface|CreateWidget "/Game/Widgets/WBP/WBP_Controls.WBP_Controls_C" self))
  (Variables|Default|SetControls _returnvalue_3)
  (bind _returnvalue_4 (UserInterface|CreateWidget "/Game/Widgets/WBP/WBP_Credits.WBP_Credits_C" self))
  (Variables|Default|SetCredits _returnvalue_4))

(event EventSetControlsHUDonScreen
  ;[0 1 0.5286] Settings, Controls and Back To Main Menu. Basically, UI Navigation Flow
  (Widget|RemovefromParent (Variables|Default|GetMenuWidget))
  (UserInterface|Viewport|AddtoViewport (Variables|Default|GetControls) 0))

(event EventSetSettingsHUDonScreen
  ;[0 1 0.5286] Settings, Controls and Back To Main Menu. Basically, UI Navigation Flow
  (Widget|RemovefromParent (Variables|Default|GetMenuWidget))
  (UserInterface|Viewport|AddtoViewport (Variables|Default|GetMenuSettings) 0))

(event EventShowCreditsonScreen
  ;[0 1 0.5286] Settings, Controls and Back To Main Menu. Basically, UI Navigation Flow
  (Widget|RemovefromParent (Variables|Default|GetMenuWidget))
  (UserInterface|Viewport|AddtoViewport (Variables|Default|GetCredits) 0))

(fn ConstructionScript)